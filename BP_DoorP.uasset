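; BP_DoorP is a puzzle door that swings its Cube between 0 and 90 degrees of world yaw using a timeline.
; On BeginPlay it binds puzzle evaluation to Button2's status change; the matching Button1 binding is disconnected and never runs.
; Each evaluation that finds both buttons pressed hits a FlipFlop, alternately playing and reversing the timeline.
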(event Custom|Evaluate%20puzzle
  ;[0.15 0.15 0.15 0.5] Interact
  (if (and (Variables|/Game/Blueprints/Platformer/BP_ButtonVisualB.BP_ButtonVisualB_C|GetIsPressed (Variables|Default|GetButton1)) (Variables|/Game/Blueprints/Platformer/BP_ButtonVisualR.BP_ButtonVisualR_C|GetIsPressed (Variables|Default|GetButton2)))
    (Utilities|FlowControl|FlipFlop
      (:A
        (bind _alpha (Timeline|TL_Door Play)
          (:Update
            (Transformation|SetWorldRotation (Variables|Default|GetCube) (Math|Rotator|MakeRotator 0.0 0.0 (Math|Float|Lerp 0.0 9e+01 _alpha)) false false))))
      (:B
        (Timeline|TL_Door Reverse)))))

(event EventBeginPlay
  (bind _button2 (Variables|Default|GetButton2))
  (Utilities|IsValid _button2
    (:Is%20Valid
      (EventDispatchers|BindEventtoStatusChanged _button2 (delegate Custom|Evaluate%20puzzle)))))

(fn ConstructionScript)