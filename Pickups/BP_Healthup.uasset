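; BP_Healthup is a health pickup that restores a fixed amount of health to the player or an enemy that walks into it.
; A Box overlap event checks the overlapping actor's Player and Enemy tags in sequence.
; It casts to BP_PlayerCharacter or BP_Enemy, calls Healthup or Heal respectively, then destroys itself.
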(event OnComponentBeginOverlap(Box)
  (params (OverlappedComponent :type Primitive%20Component%20Object%20Reference) (OtherActor :type Actor%20Object%20Reference) (OtherComp :type Primitive%20Component%20Object%20Reference) (OtherBodyIndex :type Integer) (bFromSweep :type Boolean) (SweepResult :type Hit%20Result%20Structure%20%28by%20ref%29))
  ;[0.15 0.15 0.15 0.5] Player Healthup
  (Utilities|FlowControl|Sequence
    (:then_0
      (if (Actor|ActorHasTag OtherActor "Player")
        (bind _asbp_player_character (Utilities|Casting|CastToBP_PlayerCharacter OtherActor))
        (Default|Healthup _asbp_player_character 25.0)
        (Actor|DestroyActor)))
    (:then_1
      ;[0.15 0.15 0.15 0.5] Enemy Healthup
      (if (Actor|ActorHasTag OtherActor "Enemy")
        (bind _asbp_enemy (Utilities|Casting|CastToBP_Enemy OtherActor))
        (Default|Heal _asbp_enemy 25.0)
        (Actor|DestroyActor)))))

(fn ConstructionScript)