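; BP_Beast is an enemy character that takes damage, credits the player with a kill on death and destroys itself.
; It gets a random name from GM_Gamemode, shown while the player overlaps NameRender.
; Tick updates a camera-facing health bar, while RotateText is a self-repeating delay loop that yaws the visible name.
; Custom events provide capped healing, a timed speed multiplier and a sphere-trace attack that damages a given target.
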(event OnComponentBeginOverlap(NameRender)
  (params (OverlappedComponent :type Primitive%20Component%20Object%20Reference) (OtherActor :type Actor%20Object%20Reference) (OtherComp :type Primitive%20Component%20Object%20Reference) (OtherBodyIndex :type Integer) (bFromSweep :type Boolean) (SweepResult :type Hit%20Result%20Structure%20%28by%20ref%29))
  ;[0.15 0.15 0.15 0.5] Name Rendering
  (Variables|Default|SetCharcter%20Ref OtherActor)
  (if (Actor|ActorHasTag OtherActor "Player")
    (Rendering|SetVisibility (Variables|Default|GetTextRender) true false)))

(event OnComponentEndOverlap(NameRender)
  (params (OverlappedComponent :type Primitive%20Component%20Object%20Reference) (OtherActor :type Actor%20Object%20Reference) (OtherComp :type Primitive%20Component%20Object%20Reference) (OtherBodyIndex :type Integer))
  ;[0.15 0.15 0.15 0.5] Name Rendering
  (if (Actor|ActorHasTag OtherActor "Player")
    (Rendering|SetVisibility (Variables|Default|GetTextRender) false false)))

(event Custom|Heal
  (params (New%20Health :type Float%20%28double-precision%29))
  ;[0.15 0.15 0.15 0.5] Healthup
  (Variables|Default|SetHealth (+ (Variables|Default|GetHealth) New%20Health))
  (if (> (Variables|Default|GetHealth) 1e+02)
    (Variables|Default|SetHealth 1e+02)))

(event Custom|Rotate%20Text
  ;[0.15 0.15 0.15 0.5] Name Rotation
  (if (Rendering|IsVisible (Variables|Default|GetTextRender))
    (Transformation|SetWorldRotation (Variables|Default|GetTextRender) (Math|Rotator|MakeRotator 0.0 0.0 (.yaw (Math|Rotator|FindLookatRotation (Transformation|GetActorLocation) (Transformation|GetActorLocation (Variables|Default|GetCharcter%20Ref))))) false false)
    (Utilities|FlowControl|Delay 0.01)
    (CallFunction|RotateText)))

(event Custom|Speed
  (params (Speed%20Multiplier :type Float%20%28double-precision%29))
  (bind _charactermovement (Variables|Character|GetCharacterMovement))
  ;[0.15 0.15 0.15 0.5] Speedup
  (Variables|/Script/Engine.CharacterMovementComponent|SetMaxWalkSpeed _charactermovement (* Speed%20Multiplier (Variables|Default|GetOriginal%20Speed)))
  (Utilities|FlowControl|Delay 1e+01)
  (Variables|/Script/Engine.CharacterMovementComponent|SetMaxWalkSpeed _charactermovement (Variables|Default|GetOriginal%20Speed)))

(event EventTick
  (params (DeltaSeconds :type Float%20%28single-precision%29))
  (bind _healthbar_widget (Variables|Default|GetHealthBar%20Widget))
  ;[0.15 0.15 0.15 0.5] Enemy Healthbar
  (bind _aswbp_enemy_hud (Utilities|Casting|CastToWBP_EnemyHUD (UserInterface|GetWidget (Variables|Default|GetHealthBar%20Widget))))
  (Progress|SetPercent (Variables|/Game/Blueprints/Enemy/WBP_EnemyHUD.WBP_EnemyHUD_C|GetEnemyHealth _aswbp_enemy_hud) (/ (Variables|Default|GetHealth) 1e+02))
  (Transformation|SetWorldRotation _healthbar_widget (Math|Rotator|FindLookatRotation (Transformation|GetWorldLocation _healthbar_widget) (Transformation|GetWorldLocation (Variables|/Script/Engine.PlayerCameraManager|GetTransformComponent (Game|GetPlayerCameraManager 0)))) false false))

(event EventBeginPlay
  ;[0.15 0.15 0.15 0.5] Shoot
  ;[0.15 0.15 0.15 0.5] Name Enemy
  (bind _asgm_gamemode (Utilities|Casting|CastToGM_Gamemode (Game|GetGameMode)))
  (Rendering|Components|TextRender|SetText (Variables|Default|GetTextRender) (Utilities|Array|Get(acopy) (Variables|/Game/Blueprints/GM_Gamemode.GM_Gamemode_C|GetEnemyNames _asgm_gamemode) (Math|Random|RandomInteger (Utilities|Array|Length (Variables|/Game/Blueprints/GM_Gamemode.GM_Gamemode_C|GetEnemyNames _asgm_gamemode)))))
  ;[0.15 0.15 0.15 0.5] Set Speed
  (Variables|/Script/Engine.CharacterMovementComponent|SetMaxWalkSpeed (Variables|Character|GetCharacterMovement) 2.5e+02))

(event EventAttack
  (params (TargetActor :type Actor%20Object%20Reference))
  (bind _returnvalue (Transformation|GetActorLocation))
  (bind (_outhits _returnvalue_2) (Collision|MultiSphereTraceForObjects _returnvalue _returnvalue 2e+02 (Utilities|Array|MakeArray "ObjectTypeQuery3") false 0 "ForDuration"))
  (if _returnvalue_2
    (bind _array_element (Utilities|Array|ForEachLoopwithBreak _outhits :!label _label)
      (:LoopBody
        (if (== TargetActor (.HitActor (Collision|BreakHitResult _array_element)))
          (Game|Damage|ApplyDamage (.HitActor (Collision|BreakHitResult _array_element)) 1e+01 0 0)
          (goto _label Break))))))

(event Game|Damage|EventAnyDamage
  (params (Damage :type Float%20%28single-precision%29) (DamageType :type Damage%20Type%20Object%20Reference) (InstigatedBy :type Controller%20Object%20Reference) (DamageCauser :type Actor%20Object%20Reference))
  ;[0.15 0.15 0.15 0.5] Health
  (bind _output_get (Variables|Default|SetHealth (- (Variables|Default|GetHealth) Damage)))
  (if (<= _output_get 0.0)
    (Utilities|FlowControl|Sequence
      (:then_0
        ;[0.15 0.15 0.15 0.5] Kill Counter
        (bind _asbp_player_character (Utilities|Casting|CastToBP_PlayerCharacter (Game|GetPlayerCharacter 0)))
        (Math|Integer|IncrementInt (Variables|/Game/Blueprints/BP_PlayerCharacter.BP_PlayerCharacter_C|GetKills _asbp_player_character)))
      (:then_1
        (Actor|DestroyActor)))))

(fn ConstructionScript)