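; BP_Turret is a destructible enemy turret that fires projectiles on a looping timer.
; BeginPlay starts the timer, which spawns a BP_Baseprojectile at the EnemyArrow transform.
; Damage lowers Health, and at zero it increments the player character's Kills and destroys the turret.
; Tick updates the world-space health bar widget and rotates it to face the player camera.
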(event Custom|Shoot
  ;[0.15 0.15 0.15 0.5] Shoot
  (Game|SpawnActorfromClass "/Game/Blueprints/BP_Baseprojectile.BP_Baseprojectile_C" (Transformation|GetWorldTransform (Variables|Default|GetEnemy%20arrow)) "Undefined" "MultiplyWithRoot" 0 0))

(event EventTick
  (params (DeltaSeconds :type Float%20%28single-precision%29))
  (bind _healthbar_widget (Variables|Default|GetHealthBar%20Widget))
  ;[0.15 0.15 0.15 0.5] Enemy Healthbar
  (bind _aswbp_enemy_hud (Utilities|Casting|CastToWBP_EnemyHUD (UserInterface|GetWidget (Variables|Default|GetHealthBar%20Widget))))
  (Progress|SetPercent (Variables|/Game/Blueprints/Enemy/WBP_EnemyHUD.WBP_EnemyHUD_C|GetEnemyHealth _aswbp_enemy_hud) (/ (Variables|Default|GetHealth) 1e+02))
  (Transformation|SetWorldRotation _healthbar_widget (Math|Rotator|FindLookatRotation (Transformation|GetWorldLocation _healthbar_widget) (Transformation|GetWorldLocation (Variables|/Script/Engine.PlayerCameraManager|GetTransformComponent (Game|GetPlayerCameraManager 0)))) false false))

(event EventBeginPlay
  ;[0.15 0.15 0.15 0.5] Shoot
  (Utilities|Time|SetTimerbyEvent (delegate Custom|Shoot) 4.0 true))

(event Game|Damage|EventAnyDamage
  (params (Damage :type Float%20%28single-precision%29) (DamageType :type Damage%20Type%20Object%20Reference) (InstigatedBy :type Controller%20Object%20Reference) (DamageCauser :type Actor%20Object%20Reference))
  ;[0.15 0.15 0.15 0.5] Health
  (bind _output_get (Variables|Default|SetHealth (- (Variables|Default|GetHealth) Damage)))
  (if (<= _output_get 0.0)
    (Utilities|FlowControl|Sequence
      (:then_0
        ;[0.15 0.15 0.15 0.5] Kill Counter
        (bind _asbp_player_character (Utilities|Casting|CastToBP_PlayerCharacter (Game|GetPlayerCharacter 0)))
        (Math|Integer|IncrementInt (Variables|/Game/Blueprints/BP_PlayerCharacter.BP_PlayerCharacter_C|GetKills _asbp_player_character)))
      (:then_1
        (Actor|DestroyActor)))))

(fn ConstructionScript)